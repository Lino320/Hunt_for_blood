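; Ranged enemy character that casts single or multiple projectiles and damages the player on contact.
; Behavior-tree attack calls feed an indexed montage combo that only dispatches the first two of four attacks, with an aim event turning a mesh toward the player.
; AnyDamage lowers Health and plays reaction montages, while Tick destroys the actor at zero.
; A separate damage event uses an attributes object to trigger ragdoll death and delayed destruction.
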(event `self.ReceiveTick`
  (params (DeltaSeconds :type "Float (single-precision)"))
  (if (<= (`self.Health`) 0.0)
    (`self.K2_DestroyActor`)))

(event `self.ReceiveAnyDamage`
  (params (Damage :type "Float (single-precision)") (DamageType :type "DamageType Object Reference") (InstigatedBy :type "Controller Object Reference") (DamageCauser :type "Actor Object Reference"))
  (`/Engine/EditorBlueprintResources/StandardMacros.DoOnce` false :!label _label
    (:`Completed`
      (bind _output_get (set `self.Health` (- (`self.Health`) Damage)))
      (if (<= _output_get 0.0)
        (`self.PlayAnimMontage` "/Game/Enemy/DeathDie.DeathDie")
        (else
          (bind _returnvalue (`self.PlayAnimMontage` "/Game/Enemy/FlyingBack.FlyingBack"))
          (`KismetSystemLibrary.Delay` _returnvalue)
          (goto _label :!via `Reset`))))))

(event `Attack 1`
  ;[1 1 1] Combat system
  ;;[1 1 1] Attack 1
  (`/Engine/EditorBlueprintResources/StandardMacros.DoOnce` false :!label _label_2
    (:`Completed`
      (`KismetSystemLibrary.Delay` 0.2)
      (`|PlayMontage` (`self.Mesh`) "/Game/AI_Advanced/Boss/Animation-Equipment/CastingSpell_1__UE_Montage.CastingSpell_1__UE_Montage" (`self.Attack animation speed`)
        (:`then`
          (`|SpawnActorFromClass` "/Game/AI_Advanced/Proyectile.Proyectile_C" (`KismetMathLibrary.MakeTransform` (`SceneComponent.K2_GetComponentLocation` (`self.Scene`))) "AlwaysSpawn" "MultiplyWithRoot" null null)
          (set `self.Atack Index` 1)
          (goto _label_2 :!via `Reset`))))))

(event `AttackComboEventCall_BT`
  ;[1 1 1] Combat system
  (if (`self.Can Atack?`)
    (`self.Combo_Atack`)))

(event `Enable Investigation Icon`
  (bind _investigation_icon (`self.Investigation Icon`))
  (`/Engine/EditorBlueprintResources/StandardMacros.FlipFlop`
    (:`A`
      (`SceneComponent.SetVisibility` _investigation_icon true false))
    (:`B`
      (`SceneComponent.SetVisibility` _investigation_icon false false))))

(event `Attack 2`
  ;[1 1 1] Combat system
  ;;[1 1 1] Attack 2
  (`/Engine/EditorBlueprintResources/StandardMacros.DoOnce` false :!label _label_3
    (:`Completed`
      (`KismetSystemLibrary.Delay` 0.2)
      (`|PlayMontage` (`self.Mesh`) "/Game/AI_Advanced/Boss/Animation-Equipment/WideArmSpellCasting_1__UE_Montage.WideArmSpellCasting_1__UE_Montage" (`self.Attack animation speed`)
        (:`then`
          (set `self.Atack Index` 2)
          (goto _label_3 :!via `Reset`))
        (:`OnCompleted`
          (`|SpawnActorFromClass` "/Game/AI_Advanced/Proyectile_Multiple.Proyectile_Multiple_C" (`KismetMathLibrary.MakeTransform` (`SceneComponent.K2_GetComponentLocation` (`self.Scene`))) "AlwaysSpawn" "MultiplyWithRoot" null null))))))

(event `Combo_Atack`
  ;[1 1 1] Combat system
  ;;[1 1 1] Combo Attack
  (if (`self.Is Atacking?`)
    (set `self.Save Atacking?` true)
    (else
      (set `self.Save Atacking?` true)
      (switch `int` (`self.Atack Index`) :!label _label_4
        (:`0`
          (`self.Attack 1`))
        (:`1`
          (`self.Attack 2`))))))

(event `Attack 3`
  ;[1 1 1] Combat system
  ;;[1 1 1] Attack 3
  (`/Engine/EditorBlueprintResources/StandardMacros.DoOnce` false :!label _label_5
    (:`Completed`
      (`KismetSystemLibrary.Delay` 0.2)
      (`|PlayMontage` (`self.Mesh`) "/Game/Enemy/ComboAnim/Attack3_Montage.Attack3_Montage" (`self.Attack animation speed`)
        (:`then`
          (set `self.Atack Index` 3)
          (goto _label_5 :!via `Reset`))))))

(event `Sword_Attack_Combo`
  ;[1 1 1] Combat system
  ;;[1 1 1] Combo continue
  (if (`self.Save Atacking?`)
    (set `self.Save Atacking?` false)
    (goto _label_4)
    (else
      (`self.Stop_ComboFR`))))

(event `Attack 4`
  ;[1 1 1] Combat system
  ;;[1 1 1] Attack 4
  (`/Engine/EditorBlueprintResources/StandardMacros.DoOnce` false :!label _label_6
    (:`Completed`
      (`KismetSystemLibrary.Delay` 0.2)
      (`|PlayMontage` (`self.Mesh`) "/Game/Enemy/ComboAnim/Kick_Montage.Kick_Montage" (`self.Attack animation speed`)
        (:`then`
          (set `self.Atack Index` 4)
          (goto _label_6 :!via `Reset`))))))

(event `Stop_ComboFR`
  ;[1 1 1] Combat system
  ;;[1 1 1] Stop combo / Attack
  (set `self.Is Atacking?` false)
  (set `self.Atack Index` 0))

(event `SetAim`
  ;[1 1 1] Weapon aim
  ;;[1 1 1] Set weapon world rotation
  (`SceneComponent.K2_SetWorldRotation` (`self.Mesh`) (`KismetMathLibrary.MakeRotator` 0.0 (.pitch (`KismetMathLibrary.FindLookAtRotation` (`SceneComponent.K2_GetComponentLocation` (`self.Mesh`)) (`KismetMathLibrary.MakeVector` (.x (`self.K2_GetActorLocation` (`GameplayStatics.GetPlayerPawn` 0))) (.y (`self.K2_GetActorLocation` (`GameplayStatics.GetPlayerPawn` 0))) (+ (.z (`self.K2_GetActorLocation` (`GameplayStatics.GetPlayerPawn` 0))) 50.0)))) (.yaw (`KismetMathLibrary.FindLookAtRotation` (`SceneComponent.K2_GetComponentLocation` (`self.Mesh`)) (`KismetMathLibrary.MakeVector` (.x (`self.K2_GetActorLocation` (`GameplayStatics.GetPlayerPawn` 0))) (.y (`self.K2_GetActorLocation` (`GameplayStatics.GetPlayerPawn` 0))) (+ (.z (`self.K2_GetActorLocation` (`GameplayStatics.GetPlayerPawn` 0))) 50.0))))) false false))

(event `CustomEvent`
  (params (Damage :type "Float (single-precision)") (DamageType :type "DamageType Object Reference") (InstigatedBy :type "Controller Object Reference") (DamageCauser :type "Actor Object Reference"))
  ;[1 1 1] Aplay Damage
  (bind _is_player_dead (`/Game/AI_Advanced/Boss/AtributesForEntities_BP.Decrease Health` (`self.AtributesForEntities_BP`) Damage))
  (if _is_player_dead
    (`self.Death`)))

(event `Death`
  ;[1 1 1] Death
  (`PrimitiveComponent.SetSimulatePhysics` (`self.Mesh`) true)
  (`KismetSystemLibrary.Delay` 5.0)
  (`self.K2_DestroyActor`))

(event `self.ReceiveHit`
  (params (MyComp :type "PrimitiveComponent Object Reference") (Other :type "Actor Object Reference") (OtherComp :type "PrimitiveComponent Object Reference") (bSelfMoved :type Boolean) (HitLocation :type "Vector Structure") (HitNormal :type "Vector Structure") (NormalImpulse :type "Vector Structure") (Hit :type "HitResult Structure (by ref)"))
  (bind _instigator (`self.Instigator`))
  ;[1 1 1] Takes damage
  (set `self.other` Other)
  (bind _asbp_third_person_character (cast `/Game/ThirdPerson/Blueprints/BP_ThirdPersonCharacter` (`self.other`)))
  (if (not (== _asbp_third_person_character _instigator))
    (`/Engine/EditorBlueprintResources/StandardMacros.DoOnce` false :!label _label_7
      (:`Completed`
        (`GameplayStatics.ApplyDamage` _asbp_third_person_character 10.0 (`self.GetController` _instigator) self)
        (`KismetSystemLibrary.Delay` 2.0)
        (goto _label_7 :!via `Reset`)))))

(fn `Attack`
  (returns (`Animation Duration` :type "Float (double-precision)"))
  (`self.AttackComboEventCall_BT`)
  (return 0.4))

(fn `StopCombo`)

(fn `UserConstructionScript`)