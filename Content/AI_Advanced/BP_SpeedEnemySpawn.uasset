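; BP_SpeedEnemySpawn is a melee enemy character with montage-driven combo attacks, health and a toggleable investigation icon.
; Attack, returning a fixed duration, triggers the combo if attacking is allowed.
; An attack index selects among four DoOnce-guarded montages (the last a kick), while a saved-input flag continues or resets the chain.
; Damage plays a fly-back reaction, locking out further hits until it ends, or a death montage at zero health.
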(event `self.ReceiveAnyDamage`
  (params (Damage :type "Float (single-precision)") (DamageType :type "DamageType Object Reference") (InstigatedBy :type "Controller Object Reference") (DamageCauser :type "Actor Object Reference"))
  (`/Engine/EditorBlueprintResources/StandardMacros.DoOnce` false :!label _label
    (:`Completed`
      (bind _output_get (set `self.Health` (- (`self.Health`) Damage)))
      (if (<= _output_get 0.0)
        (`self.PlayAnimMontage` "/Game/Enemy/DeathDie.DeathDie")
        (else
          (bind _returnvalue (`self.PlayAnimMontage` "/Game/Enemy/FlyingBack.FlyingBack"))
          (`KismetSystemLibrary.Delay` _returnvalue)
          (goto _label :!via `Reset`))))))

(event `Attack 1`
  ;[1 1 1] Combat system
  ;;[1 1 1] Attack 1
  (`/Engine/EditorBlueprintResources/StandardMacros.DoOnce` false :!label _label_2
    (:`Completed`
      (`KismetSystemLibrary.Delay` 0.2)
      (`|PlayMontage` (`self.Mesh`) "/Game/Enemy/ComboAnim/Attack1_Montage.Attack1_Montage" (`self.Attack animation speed`)
        (:`then`
          (set `self.Atack Index` 1)
          (goto _label_2 :!via `Reset`))))))

(event `AttackComboEventCall_BT`
  ;[1 1 1] Combat system
  (if (`self.Can Atack?`)
    (`self.Combo_Atack`)))

(event `Enable Investigation Icon`
  (bind _investigation_icon (`self.Investigation Icon`))
  (`/Engine/EditorBlueprintResources/StandardMacros.FlipFlop`
    (:`A`
      (`SceneComponent.SetVisibility` _investigation_icon true false))
    (:`B`
      (`SceneComponent.SetVisibility` _investigation_icon false false))))

(event `Attack 2`
  ;[1 1 1] Combat system
  ;;[1 1 1] Attack 2
  (`/Engine/EditorBlueprintResources/StandardMacros.DoOnce` false :!label _label_3
    (:`Completed`
      (`KismetSystemLibrary.Delay` 0.2)
      (`|PlayMontage` (`self.Mesh`) "/Game/Enemy/ComboAnim/Attack2_Montage.Attack2_Montage" (`self.Attack animation speed`)
        (:`then`
          (set `self.Atack Index` 2)
          (goto _label_3 :!via `Reset`))))))

(event `Combo_Atack`
  ;[1 1 1] Combat system
  ;;[1 1 1] Combo Attack
  (if (`self.Is Atacking?`)
    (set `self.Save Atacking?` true)
    (else
      (set `self.Save Atacking?` true)
      (switch `int` (`self.Atack Index`) :!label _label_4
        (:`0`
          (`self.Attack 1`))
        (:`1`
          (`self.Attack 2`))
        (:`2`
          (`self.Attack 3`))
        (:`3`
          (`self.Attack 4`))))))

(event `Attack 3`
  ;[1 1 1] Combat system
  ;;[1 1 1] Attack 3
  (`/Engine/EditorBlueprintResources/StandardMacros.DoOnce` false :!label _label_5
    (:`Completed`
      (`KismetSystemLibrary.Delay` 0.2)
      (`|PlayMontage` (`self.Mesh`) "/Game/Enemy/ComboAnim/Attack3_Montage.Attack3_Montage" (`self.Attack animation speed`)
        (:`then`
          (set `self.Atack Index` 3)
          (goto _label_5 :!via `Reset`))))))

(event `Sword_Attack_Combo`
  ;[1 1 1] Combat system
  ;;[1 1 1] Combo continue
  (if (`self.Save Atacking?`)
    (set `self.Save Atacking?` false)
    (goto _label_4)
    (else
      (`self.Stop_ComboFR`))))

(event `Attack 4`
  ;[1 1 1] Combat system
  ;;[1 1 1] Attack 4
  (`/Engine/EditorBlueprintResources/StandardMacros.DoOnce` false :!label _label_6
    (:`Completed`
      (`KismetSystemLibrary.Delay` 0.2)
      (`|PlayMontage` (`self.Mesh`) "/Game/Enemy/ComboAnim/Kick_Montage.Kick_Montage" (`self.Attack animation speed`)
        (:`then`
          (set `self.Atack Index` 4)
          (goto _label_6 :!via `Reset`))))))

(event `Stop_ComboFR`
  ;[1 1 1] Combat system
  ;;[1 1 1] Stop combo / Attack
  (set `self.Is Atacking?` false)
  (set `self.Atack Index` 0))

(fn `Attack`
  (returns (`Animation Duration` :type "Float (double-precision)"))
  (`self.AttackComboEventCall_BT`)
  (return 0.4))

(fn `StopCombo`)

(fn `UserConstructionScript`)