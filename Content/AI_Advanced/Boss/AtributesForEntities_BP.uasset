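; Attribute component for the boss that holds health and stamina and drives the bars on its widget.
; On BeginPlay it waits a tick, caches the owning BOSS_TRY_BP and initializes the widget.
; Functions adjust values and maximums and push them to the UI, though regular increases refresh it only when clamped to the maximum.
; Both decrease functions return whether Health is depleted, even the stamina one, which never checks Stamina.
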(event `self.ReceiveBeginPlay`
  (bind _widgetboss (`/Game/AI_Advanced/Boss/BOSS_TRY_BP.WidgetBoss` (`self.BOSS BP`)))
  (`KismetSystemLibrary.DelayUntilNextTick`)
  (bind _asboss_try_bp (cast `/Game/AI_Advanced/Boss/BOSS_TRY_BP` (`self.GetOwner`)))
  (set `self.BOSS BP` _asboss_try_bp)
  (`ProgressBar.SetPercent` (`/Game/AI_Advanced/Boss/WB_HealthBarBOSS.StaminaBarBoss` (`/Game/AI_Advanced/Boss/BOSS_TRY_BP.WidgetBoss` (`self.BOSS BP`))) (/ (`self.Stamina`) (`self.MaxStamina`)))
  (`ProgressBar.SetPercent` (`/Game/AI_Advanced/Boss/WB_HealthBarBOSS.HealthBarBoss` _widgetboss) (/ (`self.Health`) (`self.MaxHealth`)))
  (`TextBlock.SetText` (`/Game/AI_Advanced/Boss/WB_HealthBarBOSS.HealthText` _widgetboss) (`KismetTextLibrary.Conv_DoubleToText` (`self.Health`) "HalfToEven")))

(fn `Decrease Health`
  (params (Damage :type "Float (double-precision)" :default 0.0))
  (returns (`Is Player Dead` :type Boolean))
  (bind _widgetboss (`/Game/AI_Advanced/Boss/BOSS_TRY_BP.WidgetBoss` (`self.BOSS BP`)))
  (if (not (<= (`self.Health`) 0.0))
    (bind _output_get (set `self.Health` (- (`self.Health`) Damage)))
    (`ProgressBar.SetPercent` (`/Game/AI_Advanced/Boss/WB_HealthBarBOSS.HealthBarBoss` _widgetboss) (/ _output_get (`self.MaxHealth`)))
    (`TextBlock.SetText` (`/Game/AI_Advanced/Boss/WB_HealthBarBOSS.HealthText` _widgetboss) (`KismetTextLibrary.Conv_DoubleToText` (`self.Health`) "HalfToEven"))
    (if (<= (`self.Health`) 0.0)
      _
      (else
        (return false))))
  (return true))

(fn `Decrease Stamina`
  (params (`Stamina Deployment` :type "Float (double-precision)" :default 0.0))
  (returns (`Not Stamina Left` :type Boolean))
  (if (not (<= (`self.Health`) 0.0))
    (set `self.Stamina` (- (`self.Stamina`) `Stamina Deployment`))
    (`ProgressBar.SetPercent` (`/Game/AI_Advanced/Boss/WB_HealthBarBOSS.StaminaBarBoss` (`/Game/AI_Advanced/Boss/BOSS_TRY_BP.WidgetBoss` (`self.BOSS BP`))) (/ (`self.Stamina`) (`self.MaxStamina`)))
    (if (<= (`self.Health`) 0.0)
      _
      (else
        (return false))))
  (return true))

(fn `Increase Health`
  (params (`Added Health` :type "Float (double-precision)" :default 0.0))
  (bind _widgetboss (`/Game/AI_Advanced/Boss/BOSS_TRY_BP.WidgetBoss` (`self.BOSS BP`)))
  (set `self.Health` (+ (`self.Health`) `Added Health`))
  (if (> (`self.Health`) (`self.MaxHealth`))
    (set `self.Health` (`self.MaxHealth`))
    (`ProgressBar.SetPercent` (`/Game/AI_Advanced/Boss/WB_HealthBarBOSS.HealthBarBoss` _widgetboss) (/ (`self.Health`) (`self.MaxHealth`)))
    (`TextBlock.SetText` (`/Game/AI_Advanced/Boss/WB_HealthBarBOSS.HealthText` _widgetboss) (`KismetTextLibrary.Conv_DoubleToText` (`self.Health`) "HalfToEven"))))

(fn `Increase Max Health`
  (params (`Health Incremention` :type "Float (double-precision)" :default 0.0))
  (bind _widgetboss (`/Game/AI_Advanced/Boss/BOSS_TRY_BP.WidgetBoss` (`self.BOSS BP`)))
  (set `self.MaxHealth` (+ (`self.Health`) `Health Incremention`))
  (`ProgressBar.SetPercent` (`/Game/AI_Advanced/Boss/WB_HealthBarBOSS.HealthBarBoss` _widgetboss) (/ (`self.Health`) (`self.MaxHealth`)))
  (`TextBlock.SetText` (`/Game/AI_Advanced/Boss/WB_HealthBarBOSS.HealthText` _widgetboss) (`KismetTextLibrary.Conv_DoubleToText` (`self.Health`) "HalfToEven")))

(fn `Increase Max Stamina`
  (params (`Added Stamina` :type "Float (double-precision)" :default 0.0))
  (set `self.MaxStamina` (+ (`self.MaxStamina`) `Added Stamina`))
  (`ProgressBar.SetPercent` (`/Game/AI_Advanced/Boss/WB_HealthBarBOSS.StaminaBarBoss` (`/Game/AI_Advanced/Boss/BOSS_TRY_BP.WidgetBoss` (`self.BOSS BP`))) (/ (`self.Stamina`) (`self.MaxStamina`))))

(fn `Increase Stamina`
  (params (`Increase Stamina` :type "Float (double-precision)" :default 0.0))
  (set `self.Stamina` (+ (`self.Stamina`) `Increase Stamina`))
  (if (> (`self.Stamina`) (`self.MaxStamina`))
    (set `self.Stamina` (`self.MaxStamina`))
    (`ProgressBar.SetPercent` (`/Game/AI_Advanced/Boss/WB_HealthBarBOSS.StaminaBarBoss` (`/Game/AI_Advanced/Boss/BOSS_TRY_BP.WidgetBoss` (`self.BOSS BP`))) (/ (`self.Stamina`) (`self.MaxStamina`)))))