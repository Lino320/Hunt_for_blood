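; BOSS_TRY_BP is a boss actor driven by an AI controller, apparently an experimental version judging by its name.
; Every tick, after calling the parent Tick, it casts its AI controller to BP_Contoller_BOSS and sets that controller's HealthBoss to zero.
; BeginPlay and overlap events are disabled stubs, and the construction script only calls its parent.
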(event `self.ReceiveTick`
  (params (DeltaSeconds :type "Float (single-precision)"))
  (`parent.ReceiveTick` DeltaSeconds)
  (bind _asbp_contoller_boss (cast `/Game/AI_Advanced/Boss/BP_Contoller_BOSS` (`AIBlueprintHelperLibrary.GetAIController` self)))
  (set `/Game/AI_Advanced/Boss/BP_Contoller_BOSS.Health_Boss` 0.0 _asbp_contoller_boss))

(fn `UserConstructionScript`
  (`parent.UserConstructionScript`))