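; BP_Contoller_BOSS is the boss controller, which starts the BT_AI_BOSS behavior tree on BeginPlay and manages the boss's on-screen health bar.
; Activate_Boss_Combat creates a WB_HealthBarBOSS widget and adds it to the viewport, and Deactivate_Boss_Combat removes it and clears the reference.
; While that widget is valid, Tick sets the bar's fill from current health over maximum health.
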(event `self.ReceiveBeginPlay`
  (`self.RunBehaviorTree` "/Game/AI_Advanced/Boss/BT_AI_BOSS.BT_AI_BOSS"))

(event `self.ReceiveTick`
  (params (DeltaSeconds :type "Float (single-precision)"))
  (bind _boss_health_widget (`self.Boss_Health_Widget`)
    (:`then`
      (bind _output_get (set `self.Boss_Health_Widget` _boss_health_widget))
      (`ProgressBar.SetPercent` (`/Game/AI_Advanced/Boss/WB_HealthBarBOSS.HealthBarBoss` _output_get) (/ (`self.Health_Boss`) (`self.MaxHealth_Boss`))))
    (:`else`)))

(event `Activate_Boss_Combat`
  (bind _returnvalue (`|CreateWidget` "/Game/AI_Advanced/Boss/WB_HealthBarBOSS.WB_HealthBarBOSS_C"))
  (bind _output_get (set `self.Boss_Health_Widget` _returnvalue))
  (`UserWidget.AddToViewport` _output_get 0))

(event `Deactivate_Boss_Combat`
  (`Widget.RemoveFromParent` (`self.Boss_Health_Widget`))
  (set `self.Boss_Health_Widget` null))

(fn `UserConstructionScript`
  (`parent.UserConstructionScript`))