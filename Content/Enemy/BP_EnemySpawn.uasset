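; BP_EnemySpawn is a work-in-progress melee enemy character that chases the player once PawnSensing sees them.
; FollowPlayer uses AI MoveTo, then plays a vampire-bite montage on arrival, with a random flag for an unfinished bleeding attack.
; Any damage plays hit and death montages and destroys it, since Health is forced to zero.
; The health widget is cached on BeginPlay, but its update logic is disconnected.
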(event `self.ReceiveBeginPlay`
  (bind _asenemy_health (cast `/Game/Enemy/Enemy_Health` (`WidgetComponent.GetUserWidgetObject` (`self.Widget`))))
  (bind _output_get (set `self.WidgetHealth` _asenemy_health))
  (set `self.Health` (`self.Health`)))

(event `self.ReceiveTick`
  (params (DeltaSeconds :type "Float (single-precision)"))
  (if (not (`self.isSeeingPlayer`))
    (`MovementComponent.StopMovementImmediately` (`self.CharacterMovement`))))

(event `self.PawnSensing.OnSeePawn`
  (params (Pawn :type "Pawn Object Reference"))
  (set `self.isSeeingPlayer` true)
  (`self.FollowPlayer`))

(event `FollowPlayer`
  (set `self.CanAttack` true)
  (if (`self.isSeeingPlayer`)
    (`|AIMoveTo` self (0.0 0.0 0.0) (`GameplayStatics.GetPlayerCharacter` 0) 70.0
      (:`OnSuccess`
        (if (`self.CanAttack`)
          (set `self.CanAttack` false)
          ;[1 1 1] No se porque no me va la anaimacion me toaca preguntar a william va como raro xD
          (bind _returnvalue (`self.PlayAnimMontage` "/Game/AI/SK_Mannequin_Montage_VampireBite.SK_Mannequin_Montage_VampireBite" 1.5))
          (`KismetSystemLibrary.Delay` _returnvalue)
          (set `self.CanAttack` true)
          (if (`KismetMathLibrary.RandomBool`)
            (set `self.BledingAtack` true))
          (elif (`self.BledingAtack`)
            (set `self.BledingAtack` false)
            (bind _returnvalue_2 (`self.PlayAnimMontage` null))
            (`KismetSystemLibrary.Delay` _returnvalue_2)
            (`KismetSystemLibrary.Delay` 3.0)
            (if (`KismetMathLibrary.RandomBool`)
              (set `self.BledingAtack` true))))))
    (else
      (set `self.isSeeingPlayer` false))))

(event `self.ReceiveAnyDamage`
  (params (Damage :type "Float (single-precision)") (DamageType :type "DamageType Object Reference") (InstigatedBy :type "Controller Object Reference") (DamageCauser :type "Actor Object Reference"))
  ;[1 1 1] Taking damage functional
  (set `self.Health` (`KismetMathLibrary.FClamp` (- (`self.Health`) Damage) 0.0 200.0))
  (if true
    (`KismetSystemLibrary.PrintString` "Hello")
    (`self.PlayAnimMontage` "/Game/Enemy/FlyingBack.FlyingBack")
    (bind _output_get (set `self.Health` 0.0))
    (if (<= _output_get 0.0)
      (`self.PlayAnimMontage` "/Game/Enemy/DeathDie.DeathDie")
      (`KismetSystemLibrary.Delay` 1.0)
      (`self.K2_DestroyActor`))))

(event `self.ReceiveHit`
  (params (MyComp :type "PrimitiveComponent Object Reference") (Other :type "Actor Object Reference") (OtherComp :type "PrimitiveComponent Object Reference") (bSelfMoved :type Boolean) (HitLocation :type "Vector Structure") (HitNormal :type "Vector Structure") (NormalImpulse :type "Vector Structure") (Hit :type "HitResult Structure (by ref)")))

(fn `UserConstructionScript`)