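; Enemy spawner that spawns an AI pawn on a looping timer started at BeginPlay.
; Each tick of the timer picks a random X/Y offset around the spawner at its own height.
; A chain of random threshold checks chooses among the first three EnemysToSpawn classes, weighted toward the first.
; Each check rolls a fresh number, so the odds differ from the thresholds and some cycles spawn nothing.
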(event `SpawnEnemy`
  (bind (_returnvalue_x _returnvalue_y _returnvalue_z) (`KismetMathLibrary.BreakVector` (`self.K2_GetActorLocation`)))
  (bind _returnvalue (`KismetMathLibrary.RandomIntegerInRange` 0 100))
  ;[1 1 1] Spawn enemy
  (bind _output_get (set `self.EnemySpawnLocation` (`KismetMathLibrary.MakeVector` (+ _returnvalue_x (`KismetMathLibrary.RandomFloatInRange` -500.0 500.0)) (+ _returnvalue_y (`KismetMathLibrary.RandomFloatInRange` -500.0 500.0)) _returnvalue_z)))
  (if (< _returnvalue 50)
    (`AIBlueprintHelperLibrary.SpawnAIFromClass` (`|GetArrayItem` (`self.EnemysToSpawn`)) null _output_get (struct) false null)
    (elif (and (>= _returnvalue 50) (< _returnvalue 75))
      (`AIBlueprintHelperLibrary.SpawnAIFromClass` (`|GetArrayItem` (`self.EnemysToSpawn`) 1) null (`self.EnemySpawnLocation`) (struct) false null)
      (elif (>= _returnvalue 75)
        (`AIBlueprintHelperLibrary.SpawnAIFromClass` (`|GetArrayItem` (`self.EnemysToSpawn`) 2) null (`self.EnemySpawnLocation`) (struct) false null)))))

(event `self.ReceiveBeginPlay`
  ;[1 1 1] Spawn enemy
  (`KismetSystemLibrary.K2_SetTimerDelegate` (delegate `SpawnEnemy`) 5.0 true))

(fn `UserConstructionScript`)