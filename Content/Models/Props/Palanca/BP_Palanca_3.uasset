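; BP_Palanca_3 is a lever prop that toggles between two positions when its Interaccion event fires.
; A FlipFlop alternately plays and reverses a timeline that lerps the handle mesh between two fixed relative transforms, playing a button sound each time.
; The Abajo flag records whether the lever is down.
; A branch that would send OpenDoorMessage to Puerta when Abajo is true is disconnected and never runs.
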(event `self.ReceiveTick`
  (params (DeltaSeconds :type "Float (single-precision)")))

(event `/Game/AI_Advanced/Objects/Pulsado.Interaccion`
  (params (player :type "/Game/ThirdPerson/Blueprints/BP_ThirdPersonCharacter Object Reference"))
  (`/Engine/EditorBlueprintResources/StandardMacros.FlipFlop`
    (:`A`
      (`GameplayStatics.PlaySound2D` "/Game/ThirdPerson/music/button2.button2" 1.0 1.0 0.0 null null)
      (set `self.abajo` true)
      (bind (_direction _anim_buttom) (`Timeline|Timeline` :!label _label)
        (:`Update`
          (bind (_returnvalue_location _returnvalue_rotation _returnvalue_scale) (`KismetMathLibrary.BreakTransform` (`KismetMathLibrary.TLerp` (`KismetMathLibrary.MakeTransform` (0.0 0.0 23.360049) (struct :`Roll` 90.0) (0.669621 0.669621 0.669621)) (`KismetMathLibrary.MakeTransform` (0.0 6.632143 23.360049) (struct :`Roll` 270.0) (0.669621 0.669621 0.669621)) _anim_buttom)))
          (`SceneComponent.K2_SetRelativeTransform` (`self.Palanca_palanca`) (`KismetMathLibrary.MakeTransform` _returnvalue_location _returnvalue_rotation _returnvalue_scale) false false))))
    (:`B`
      (`GameplayStatics.PlaySound2D` "/Game/ThirdPerson/music/button2.button2" 1.0 1.0 0.0 null null)
      (set `self.abajo` false)
      (goto _label :!via `Reverse`))))

(fn `UserConstructionScript`)